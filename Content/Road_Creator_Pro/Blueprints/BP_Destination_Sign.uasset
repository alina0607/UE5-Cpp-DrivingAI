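; Configurable destination road sign actor from Road Creator Pro, built entirely in the Construction Script.
; Exposed variables drive the text render and arrow decal layout, sign colors, retro-reflective materials, weathering and a diagonal red line.
; Poles are optional, and removing them disables physics.
; With physics enabled, text and arrow attach to the movable, simulated sign mesh; otherwise the physics constraint is destroyed.
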(fn `UserConstructionScript`
  (bind _sm_pole1 (`self.SM_Pole1`))
  (bind _arrow (`self.Arrow`))
  (bind _sm_sign (`self.SM_Sign`))
  (bind _textrender (`self.TextRender`))
  (bind _sm_pole1_2 (`self.SM_Pole1`))
  (bind (_text_location _text_rotation _text_scale) (`KismetMathLibrary.BreakTransform` (`self.Text`)))
  (bind _returnvalue (`KismetMathLibrary.Conv_ColorToLinearColor` (`self.Text Color`)))
  (bind _returnvalue_2 (`KismetMathLibrary.LinearColorLerp` (`KismetMathLibrary.SelectColor` _returnvalue (* _returnvalue (struct :`R` 0.8125 :`G` 0.8125 :`B` 0.8125 :`A` 1.0)) (`self.Retro-Reflective material`)) (struct :`R` 0.072917 :`G` 0.072917 :`B` 0.072917 :`A` 1.0) (* (`self.Old`) 0.5)))
  ; Downloaded from t.me/FABUE5AssetsFree
  ; Best environments, models, plugins, animations, VFX, SFX, templates for Unreal Engine
  (`|ExecutionSequence`
    (:`then_1`
      (`TextRenderComponent.K2_SetText` (`self.TextRender`) (`self.Sign Text`))
      ;;[1 1 1] Rotate Arrow
      (`SceneComponent.K2_SetRelativeTransform` (`self.Arrow Decal`) (`KismetMathLibrary.MakeTransform` (.location _arrow) (`KismetMathLibrary.MakeRotator` (+ (`KismetMathLibrary.SelectFloat` (.pitch (.rotation _arrow)) (- 180.0 (.pitch (.rotation _arrow))) (< (`KismetMathLibrary.Abs` (.roll (.rotation _arrow))) 1.0)) 90.0) 0.0 90.0) (.scale _arrow)) false false)
      ;;[1 1 1] Position Text
      (`SceneComponent.K2_SetRelativeTransform` (`self.TextRender`) (`KismetMathLibrary.MakeTransform` _text_location (`KismetMathLibrary.ComposeRotators` _text_rotation (struct :`Yaw` 90.0)) _text_scale) false false)
      (`SceneComponent.SetVisibility` (`self.Arrow Decal`) (`self.Arrow Enable`) false))
    (:`then_2`
      ;;[1 1 1] Retro-Reflective
      (if (`self.Retro-Reflective material`)
        (`PrimitiveComponent.SetMaterialByName` (`self.SM_Sign`) "Sign" "/Game/Road_Creator_Pro/Materials/Road_Signs/MI_Sign_Destination_Retro-Reflective.MI_Sign_Destination_Retro-Reflective")
        (`TextRenderComponent.SetTextMaterial` (`self.TextRender`) "/Game/Road_Creator_Pro/Materials/Road_Signs/Font/MI_Sign_Font_Retro-Reflective.MI_Sign_Font_Retro-Reflective")))
    (:`then_3`
      ;;[1 1 1] Colors
      (`TextRenderComponent.SetTextRenderColor` (`self.TextRender`) (`KismetMathLibrary.Conv_LinearColorToColor` _returnvalue_2 false))
      (`MeshComponent.SetVectorParameterValueOnMaterials` (`self.SM_Sign`) "Color Border" (`KismetMathLibrary.Conv_LinearColorToVector` _returnvalue))
      (bind _returnvalue_3 (`DecalComponent.CreateDynamicMaterialInstance` (`self.Arrow Decal`)))
      (`MaterialInstanceDynamic.SetVectorParameterValue` _returnvalue_3 "Color" _returnvalue_2)
      (`MeshComponent.SetVectorParameterValueOnMaterials` (`self.SM_Sign`) "Color Background" (`KismetMathLibrary.Conv_LinearColorToVector` (`KismetMathLibrary.Conv_ColorToLinearColor` (`self.Background Color`)))))
    (:`then_4`
      ;;[1 1 1] Poles
      (if (not (`self.Poles`))
        (set `self.Physics Enabled` false)
        (`ActorComponent.K2_DestroyComponent` (`self.SM_Pole1`))
        (`ActorComponent.K2_DestroyComponent` (`self.SM_Pole2`))))
    (:`then_5`
      ;;[1 1 1] Physics
      (if (`self.Physics Enabled`)
        (`SceneComponent.K2_AttachToComponent` (`self.TextRender`) (`self.SM_Sign`) "None" "KeepWorld" "KeepWorld" "KeepWorld" true)
        (`SceneComponent.K2_AttachToComponent` (`self.Arrow Decal`) (`self.SM_Sign`) "None" "KeepWorld" "KeepWorld" "KeepWorld" true)
        (`SceneComponent.SetMobility` (`self.SM_Sign`) "Movable")
        (`/Engine/EditorBlueprintResources/StandardMacros.IsValid` _sm_pole1_2
          (:`Is Valid`
            (`SceneComponent.SetMobility` _sm_pole1_2 "Movable")
            (`SceneComponent.SetMobility` (`self.SM_Pole2`) "Movable")
            (`PrimitiveComponent.SetSimulatePhysics` (`self.SM_Sign`) true)))
        (else
          (`ActorComponent.K2_DestroyComponent` (`self.PhysicsConstraint`)))))
    (:`then_6`
      ;;[1 1 1] Material Adjust
      (`MeshComponent.SetScalarParameterValueOnMaterials` _sm_sign "Red Line" (`KismetMathLibrary.Conv_BoolToDouble` (`self.Diagonal Red Line`)))
      (`MeshComponent.SetScalarParameterValueOnMaterials` _sm_sign "Old" (`self.Old`))
      (`/Engine/EditorBlueprintResources/StandardMacros.IsValid` _sm_pole1
        (:`Is Valid`
          (`MeshComponent.SetScalarParameterValueOnMaterials` _sm_pole1 "Old" (`self.Old`))
          (`MeshComponent.SetScalarParameterValueOnMaterials` (`self.SM_Pole2`) "Old" (`self.Old`)))))
    (:`then_7`
      ;;[1 1 1] Text Spacing
      (`TextRenderComponent.SetHorizSpacingAdjust` _textrender (`self.Text Horizontal Spacing`))
      (`TextRenderComponent.SetVertSpacingAdjust` _textrender (`self.Text Vertical Spacing`)))))