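; Lamp post actor that builds a straight row of evenly spaced street lights, with switchable lighting.
; The construction script creates instanced pole meshes for center, right and left options, plus optional cable instances stretched between neighboring posts.
; Optional spotlights and billboards spawn at each instance's mesh sockets.
; SetLights applies the on/off state and intensity to lights and pole emissive materials, while toggling billboard visibility, also via runtime switch events.
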(event `Turn Lights ON/OFF`
  (params (ON :type Boolean))
  (set `self.Lights On` ON)
  (`self.Set Lights`))

(event `/Game/Road_Creator_Pro/Blueprints/Helpers/BPI_Light_Control.Switch Lights`
  (params (ON :type Boolean))
  (`self.Turn Lights ON/OFF` ON))

(fn `Add Meshes`
  (params (`Side Offset` :type "Float (double-precision)") (Mesh :type "StaticMesh Object Reference") (`Mesh Length` :type "Float (double-precision)") (Height :type "Float (double-precision)") (Mirrored :type Boolean) (`Short Mesh` :type Boolean) (`Is Light Post` :type Boolean) (Scale :type "Float (double-precision)" :default 1.0) (`Scale WIdth Only` :type Boolean) (Vertical :type Boolean) (`Do Not Duplicate` :type Boolean) (`Is Asphalt` :type Boolean) (`Don't Cast Shadow` :type Boolean) (` Color` :type "LinearColor Structure") (`Color Parameter Name` :type Name) (Material :type "MaterialInterface Object Reference"))
  (locals (`Side Offset (Duplicate)` :type "Float (double-precision)"))
  (set `local.Side Offset (Duplicate)` (`local.Side Offset`))
  (`self.Add Static Meshes (Straight Road)` 0.0 (`local.Mesh`) (`local.Mesh Length`) (`local.Height`) (`local.Mirrored`) (`local.Is Light Post`) (`local.Scale`) false (`local.Vertical`) (`local.Is Asphalt`) (`local.Don't Cast Shadow`) (`local. Color`) (`local.Color Parameter Name`) (`local.Material`)))

(fn `Add Spot Light`
  (params (RelativeTransform :type "Transform Structure"))
  (`|ExecutionSequence`
    (:`then_0`
      (bind _returnvalue (`AddComponent|NODE_AddSpotLightComponent-0` :`RelativeTransform` RelativeTransform))
      (`KismetArrayLibrary.Array_Add` (`self.Spot Lights`) _returnvalue)
      (`LocalLightComponent.SetAttenuationRadius` _returnvalue (`self.Attenuation Radius`))
      (`LightComponentBase.SetCastShadows` _returnvalue (`self.Cast Shadows`))
      (`LightComponent.SetTemperature` _returnvalue (`self.Lights Temperature`)))
    (:`then_1`
      (if (`self.Light Billboards`)
        (bind _returnvalue_2 (`AddComponent|NODE_AddMaterialBillboardComponent-0` :`RelativeTransform` RelativeTransform))
        (`KismetArrayLibrary.Array_Add` (`self.Spot Light Billboards`) _returnvalue_2)))))

(fn `Add Static Meshes (Straight Road)`
  (params (`Side Offset` :type "Float (double-precision)") (Mesh :type "StaticMesh Object Reference") (`Mesh Length` :type "Float (double-precision)") (Height :type "Float (double-precision)") (Mirrored :type Boolean) (`Is Light Post` :type Boolean) (Scale :type "Float (double-precision)") (`Scale WIdth Only` :type Boolean) (Vertical :type Boolean) (`Is Asphalt` :type Boolean) (`Don't Cast Shadow` :type Boolean) (Color :type "LinearColor Structure") (`Color Parameter Name` :type Name) (Material :type "MaterialInterface Object Reference"))
  (locals (`Side Offset local` :type "Float (double-precision)") (`ISM Component` :type "InstancedStaticMeshComponent Object Reference"))
  (bind _scale (`local.Scale`))
  (bind _color (`local.Color`))
  (bind (_returnvalue_roll _returnvalue_pitch) (`KismetMathLibrary.BreakRotator` (`SceneComponent.K2_GetComponentRotation` (`local.ISM Component`))))
  (bind _returnvalue (select `bool` (`local.Mirrored`) :`false` -1.0 :`true` 1.0))
  (set `local.Side Offset local` `Side Offset`)
  ;[1 1 1] Setup ISM
  (bind _returnvalue_2 (`AddComponent|NODE_AddInstancedStaticMeshComponent-0`))
  (set `local.ISM Component` _returnvalue_2)
  (`StaticMeshComponent.SetStaticMesh` (`local.ISM Component`) (`local.Mesh`))
  (`|ExecutionSequence`
    (:`then_0`
      ;[1 1 1] Add ISM Instances
      (for _index (range (`self.Number of Posts`))
        (`InstancedStaticMeshComponent.AddInstance` (`local.ISM Component`) (`KismetMathLibrary.MakeTransform` (`KismetMathLibrary.MakeVector` (* (+ (`KismetMathLibrary.Conv_IntToDouble` _index) 0.0) (* (`self.Lights Spacing, m`) 100.0)) (`local.Side Offset local`) (`local.Height`)) (`KismetMathLibrary.MakeRotator` (* _returnvalue_roll _returnvalue) (* _returnvalue _returnvalue_pitch) (`KismetMathLibrary.SelectFloat` 180.0 0.0 (`local.Mirrored`))) (`KismetMathLibrary.MakeVector` _scale _scale _scale)) false)))
    (:`then_1`
      (if (`local.Is Light Post`)
        (`KismetArrayLibrary.Array_Add` (`self.Light Posts`) (`local.ISM Component`))))
    (:`then_3`
      (if (`local.Don't Cast Shadow`)
        (`PrimitiveComponent.SetCastShadow` (`local.ISM Component`) false)))
    (:`then_5`
      (if (!= (struct) _color)
        (`MeshComponent.SetVectorParameterValueOnMaterials` (`local.ISM Component`) (`local.Color Parameter Name`) (`KismetMathLibrary.Conv_LinearColorToVector` _color))))))

(fn `Set Lights`
  (bind _lights_intensity (`self.Lights Intensity`))
  (bind _lights_on (`self.Lights On`))
  (for _array_element (`self.Spot Lights`)
    (`SceneComponent.SetVisibility` _array_element _lights_on false)
    (`LightComponent.SetIntensity` _array_element (* _lights_intensity 15000.0)))
  (for _array_element_2 (`self.Light Posts`)
    (`MeshComponent.SetScalarParameterValueOnMaterials` _array_element_2 "emissive" (* (`KismetMathLibrary.Conv_BoolToDouble` _lights_on) _lights_intensity 10.0)))
  (for _array_element_3 (`self.Spot Light Billboards`)
    (`SceneComponent.SetVisibility` _array_element_3 (`self.Lights On`) false)))

(fn `UserConstructionScript`
  (bind _light_posts_height__cm (`self.Light Posts Height, cm`))
  (bind _lamp_post_side_offset (`self.Lamp Post side offset`))
  (bind _returnvalue (* (`self.Lights Spacing, m`) 100.0))
  (`|ExecutionSequence`
    (:`then_0`
      (`|ExecutionSequence`
        (:`then_0`
          (if (`self.💡 Lamp Posts C`)
            (`self.Add Meshes` 0.0 "/Game/Road_Creator_Pro/Meshes/Lampposts/SM_Outdoor_Pole_Light_High_2_Lamps.SM_Outdoor_Pole_Light_High_2_Lamps" _returnvalue _light_posts_height__cm false true true 1.0 false true true)))
        (:`then_1`
          (if (`self.💡 Lamp Posts R`)
            (`self.Add Meshes` _lamp_post_side_offset "/Game/Road_Creator_Pro/Meshes/Lampposts/SM_Outdoor_Pole_Light.SM_Outdoor_Pole_Light" _returnvalue _light_posts_height__cm true true true 1.0 false true)))
        (:`then_2`
          (if (`self.💡 Lamp Posts L`)
            (`self.Add Meshes` (* _lamp_post_side_offset -1.0) "/Game/Road_Creator_Pro/Meshes/Lampposts/SM_Outdoor_Pole_Light.SM_Outdoor_Pole_Light" _returnvalue _light_posts_height__cm false true true 1.0 false true)))))
    (:`then_1`
      (`|ExecutionSequence`
        (:`then_0`
          (if (not (`self.Add Spot Light Sources`))
            (set `self.Lights On` false)))
        (:`then_1`
          (if (`self.Cables between Lightposts`)
            (bind _returnvalue_2 (`AddComponent|NODE_AddInstancedStaticMeshComponent-5`))
            (set `self.Cables ISM` _returnvalue_2)))
        (:`then_2`
          (for _array_element (`self.Light Posts`)
            (for _index (range (`InstancedStaticMeshComponent.GetInstanceCount` _array_element))
              (`|ExecutionSequence`
                (:`then_0`
                  ;[1 1 1] Add Spot Light Sources
                  (if (`self.Add Spot Light Sources`)
                    (for _array_element_2 (`SceneComponent.GetAllSocketNames` _array_element)
                      (bind _outinstancetransform (`InstancedStaticMeshComponent.GetInstanceTransform` _array_element _index false))
                      (`self.Add Spot Light` (`KismetMathLibrary.ComposeTransforms` (`SceneComponent.GetSocketTransform` _array_element _array_element_2 "RTS_Component") (`KismetMathLibrary.MakeTransform` (.location _outinstancetransform) (.rotation _outinstancetransform)))))))
                (:`then_1`
                  ;[1 1 1] Add Cables
                  (if (and (!= _index 0) (`self.Cables between Lightposts`))
                    (bind _outinstancetransform_2 (`InstancedStaticMeshComponent.GetInstanceTransform` _array_element _index false))
                    (bind _outinstancetransform_3 (`InstancedStaticMeshComponent.GetInstanceTransform` _array_element (- _index 1) false))
                    (`InstancedStaticMeshComponent.AddInstance` (`self.Cables ISM`) (`KismetMathLibrary.MakeTransform` (+ (.location _outinstancetransform_2) (0.0 0.0 700.0)) (`KismetMathLibrary.ComposeRotators` (struct :`Yaw` 90.0) (`KismetMathLibrary.FindLookAtRotation` (.location _outinstancetransform_3) (.location _outinstancetransform_2))) (`KismetMathLibrary.MakeVector` 1.0 (/ (`KismetMathLibrary.Vector_Distance` (.location _outinstancetransform_2) (.location _outinstancetransform_3)) 1600.0) 1.0)) false)))))))))
    (:`then_3`
      (`self.Set Lights`))))