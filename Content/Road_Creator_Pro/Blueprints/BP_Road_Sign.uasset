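; Configurable road sign actor from Road Creator Pro that builds a pole with a main sign and optional second and rear signs in its construction script.
; It scales the pole by height, can mirror the main sign, and attaches extra signs to the pole's "Sign" socket.
; Disabling physics removes the constraint and makes meshes static.
; Options add an "Old" material look or retro-reflective materials, choosing EU or US by mesh name.
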(fn `Change Material to Retro- Reflective`
  (params (Mesh :type "StaticMeshComponent Object Reference"))
  (`PrimitiveComponent.SetMaterial` Mesh 1 (select `bool` (`KismetStringLibrary.Contains` (`KismetSystemLibrary.GetObjectName` (`StaticMeshComponent.StaticMesh` Mesh)) "_EU_") :`false` "/Game/Road_Creator_Pro/Materials/Road_Signs/MI_Sign_US_Retro-Reflective.MI_Sign_US_Retro-Reflective" :`true` "/Game/Road_Creator_Pro/Materials/Road_Signs/MI_Sign_EU_Retro-Reflective_.MI_Sign_EU_Retro-Reflective_" :!type "MaterialInterface Object Reference")))

(fn `UserConstructionScript`
  (locals (Scale :type "Vector Structure" :default (0.0 0.0 0.0)))
  (bind _second_sign_component (`self.Second Sign Component`))
  (bind _sm_sign (`self.SM_Sign`))
  (bind _second_sign_component_2 (`self.Second Sign Component`))
  (bind _second_sign (`self.Second Sign`))
  (bind _sign_scale (`self.Sign Scale`))
  (bind _rear_sign (`self.Rear Sign`))
  (bind _rear_sign_component (`self.Rear Sign Component`))
  (bind _rear_sign_component_2 (`self.Rear Sign Component`))
  (bind _rear_sign_2 (`self.Rear Sign`))
  (`|ExecutionSequence`
    (:`then_0`
      ;[1 1 1] Set Sign and Height
      (`StaticMeshComponent.SetStaticMesh` (`self.SM_Sign`) (`self.Sign Mesh`))
      (`SceneComponent.SetRelativeScale3D` (`self.SM_Pole`) (`KismetMathLibrary.MakeVector` 1.0 1.0 (/ (`self.Height`) 250.0)))
      (bind _output_get (set `local.Scale` (`KismetMathLibrary.MakeVector` (* (`KismetMathLibrary.SelectFloat` -1.0 1.0 (`self.Mirror Sign`)) _sign_scale) _sign_scale _sign_scale)))
      (`SceneComponent.SetWorldScale3D` (`self.SM_Sign`) _output_get))
    (:`then_1`
      ;[1 1 1] Add Second Sign
      (`/Engine/EditorBlueprintResources/StandardMacros.IsValid` _second_sign
        (:`Is Valid`
          (bind _returnvalue (`AddComponent|NODE_AddStaticMeshComponent-0` :`RelativeTransform` (`KismetMathLibrary.MakeTransform` (`KismetMathLibrary.MakeVector` 0.0 0.0 (* (`self.Second Sign Offset Down`) -1.0)) (struct) (`local.Scale`))))
          (bind _output_get_2 (set `self.Second Sign Component` _returnvalue))
          (`StaticMeshComponent.SetStaticMesh` _output_get_2 _second_sign)
          (`SceneComponent.K2_AttachToComponent` _output_get_2 (`self.SM_Pole`) "Sign" "KeepRelative" "KeepRelative" "KeepRelative" true))))
    (:`then_2`
      ;[1 1 1] Add Rear Sign
      (`/Engine/EditorBlueprintResources/StandardMacros.IsValid` _rear_sign
        (:`Is Valid`
          (bind _returnvalue_2 (`AddComponent|NODE_AddStaticMeshComponent-1` :`RelativeTransform` (`KismetMathLibrary.MakeTransform` (0.0 -9.0 0.0) (struct :`Yaw` 180.0) (`local.Scale`))))
          (bind _output_get_3 (set `self.Rear Sign Component` _returnvalue_2))
          (`StaticMeshComponent.SetStaticMesh` _output_get_3 _rear_sign)
          (`SceneComponent.K2_AttachToComponent` _output_get_3 (`self.SM_Pole`) "Sign" "KeepRelative" "KeepRelative" "KeepRelative" true))))
    (:`then_3`
      ;[1 1 1] Physics
      (if (not (`self.Physics Enabled`))
        (`ActorComponent.K2_DestroyComponent` (`self.PhysicsConstraint`))
        (`SceneComponent.SetMobility` (`self.SM_Pole`) "Static")
        (`SceneComponent.SetMobility` (`self.SM_Sign`) "Static")
        (`|ExecutionSequence`
          (:`then_0`
            (`/Engine/EditorBlueprintResources/StandardMacros.IsValid` _second_sign_component
              (:`Is Valid`
                (`SceneComponent.SetMobility` _second_sign_component "Static"))))
          (:`then_1`
            (`/Engine/EditorBlueprintResources/StandardMacros.IsValid` _rear_sign_component
              (:`Is Valid`
                (`SceneComponent.SetMobility` _rear_sign_component "Static")))))))
    (:`then_4`
      ;[1 1 1] Retro-Reflective and Old
      (`|ExecutionSequence`
        (:`then_0`
          (if (`self.Retro-Reflective material`)
            (`self.Change Material to Retro- Reflective` _sm_sign)
            (`/Engine/EditorBlueprintResources/StandardMacros.IsValid` (`self.Second Sign`)
              (:`Is Valid`
                (`self.Change Material to Retro- Reflective` _second_sign_component_2))
              (:`Is Not Valid`
                _))
            (`/Engine/EditorBlueprintResources/StandardMacros.IsValid` _rear_sign_2
              (:`Is Valid`
                (`self.Change Material to Retro- Reflective` _rear_sign_component_2)))))
        (:`then_1`
          (`MeshComponent.SetScalarParameterValueOnMaterials` _sm_sign "Old" (`self.Old`))
          (`MeshComponent.SetScalarParameterValueOnMaterials` (`self.SM_Pole`) "Old" (`self.Old`))
          (`/Engine/EditorBlueprintResources/StandardMacros.IsValid` (`self.Second Sign`)
            (:`Is Valid`
              (`MeshComponent.SetScalarParameterValueOnMaterials` _second_sign_component_2 "Old" (`self.Old`)))
            (:`Is Not Valid`
              _))
          (`/Engine/EditorBlueprintResources/StandardMacros.IsValid` _rear_sign_2
            (:`Is Valid`
              (`MeshComponent.SetScalarParameterValueOnMaterials` _rear_sign_component_2 "Old" (`self.Old`)))))))))