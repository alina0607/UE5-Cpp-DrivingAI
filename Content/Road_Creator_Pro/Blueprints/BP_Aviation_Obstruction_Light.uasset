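; Aviation obstruction warning light actor from Road Creator Pro that can be switched on or off.
; The construction script creates a dynamic material instance for the billboard glow and applies the initial state.
; TurnON, TurnOFF and SwitchLights set the On flag and call SetLight.
; SetLight toggles billboard visibility and scales its brightness and the mesh's emissive from Intensity, zeroing the emissive when off.
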(event `Turn ON`
  (set `self.On` true)
  (`self.Set Light`))

(event `Turn OFF`
  (set `self.On` false)
  (`self.Set Light`))

(event `/Game/Road_Creator_Pro/Blueprints/Helpers/BPI_Light_Control.Switch Lights`
  (params (ON :type Boolean))
  (if ON
    (`self.Turn ON`)
    (else
      (`self.Turn OFF`))))

(fn `Set Light`
  (bind _intensity (`self.Intensity`))
  (bind _on (`self.On`))
  (`SceneComponent.SetVisibility` (`self.MaterialBillboard`) _on false)
  (`MaterialInstanceDynamic.SetScalarParameterValue` (`self.Billboard Mat`) "Brightness" (* _intensity 50.0))
  (`MeshComponent.SetScalarParameterValueOnMaterials` (`self.SM_Aviation_Obstruction_Light`) "Emissive" (* (`KismetMathLibrary.Conv_BoolToDouble` _on) _intensity 5.0)))

(fn `UserConstructionScript`
  (bind _returnvalue (`PrimitiveComponent.CreateDynamicMaterialInstance` (`self.MaterialBillboard`) 0 null "None"))
  (set `self.Billboard Mat` _returnvalue)
  (`self.Set Light`))