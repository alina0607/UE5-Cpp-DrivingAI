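; Editor placement actor that snaps a junction mesh to the side of the nearest BP_Road_Creator road.
; The construction script finds the closest point on nearby spline or straight roads, stepping along the spline segment for precision.
; It derives side, offset and rotation from the road, applies mirroring, width and pitch, and copies asphalt material and wetness.
; ConvertToStaticMesh replaces the actor with a StaticMeshActor, carrying over mesh, transform and asphalt material.
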(fn `Convert to Static Mesh`
  (bind _asphalt_material (`self.Asphalt Material`))
  (`|ExecutionSequence`
    (:`then_0`
      (bind _returnvalue (`|SpawnActorFromClass` "/Script/Engine.StaticMeshActor" (`KismetMathLibrary.MakeTransform` (`self.Mesh Location`) (`self.Mesh Rotation`) (`self.Mesh Scale`)) "AlwaysSpawn" "MultiplyWithRoot" null null))
      (`StaticMeshComponent.SetStaticMesh` (`StaticMeshActor.StaticMeshComponent` _returnvalue) (`self.Mesh`))
      (`/Engine/EditorBlueprintResources/StandardMacros.IsValid` _asphalt_material
        (:`Is Valid`
          (`PrimitiveComponent.SetMaterial` (`StaticMeshActor.StaticMeshComponent` _returnvalue) 0 _asphalt_material))))
    (:`then_1`
      (`self.K2_DestroyActor`))))

(fn `Find closest Road`
  (locals (`Min Distance` :type "Float (double-precision)" :default 100000.0) (`Current Min Distance` :type "Float (double-precision)" :default 0.0) (`Current Road` :type "/Game/Road_Creator_Pro/Blueprints/BP_Road_Creator Object Reference") (`Current Closest Location` :type "Vector Structure" :default (0.0 0.0 0.0)))
  (bind _returnvalue (`self.GetTransform` (`local.Current Road`)))
  (bind _returnvalue_x (`KismetMathLibrary.BreakVector` (`KismetMathLibrary.InverseTransformLocation` _returnvalue (`self.K2_GetActorLocation`))))
  (bind _outactors (`KismetSystemLibrary.SphereOverlapActors` (`self.K2_GetActorLocation`) 5000.0 (`|MakeArray` "ObjectTypeQuery1" :!type "EObjectTypeQuery Enum") "/Game/Road_Creator_Pro/Blueprints/BP_Road_Creator.BP_Road_Creator_C"))
  (for _array_element _outactors
    (bind _asbp_road_creator (cast `/Game/Road_Creator_Pro/Blueprints/BP_Road_Creator` _array_element))
    (set `local.Current Road` _asbp_road_creator)
    (bind _output_get (set `self.Road Uses Spline` (`/Game/Road_Creator_Pro/Blueprints/BP_Road_Creator.Use Spline` (`local.Current Road`))))
    (if _output_get
      (bind (_distance_on_spline _closest_location) (`self.Search Closest Point On Spline` (`/Game/Road_Creator_Pro/Blueprints/BP_Road_Creator.Input Spline` (`local.Current Road`)) (`self.K2_GetActorLocation`) 10.0))
      (bind _output_get_2 (set `local.Current Closest Location` _closest_location))
      (set `local.Current Min Distance` (`KismetMathLibrary.Vector_Distance` (`self.K2_GetActorLocation`) _output_get_2))
      (else
        (bind _output_get_3 (set `local.Current Closest Location` (`KismetMathLibrary.TransformLocation` _returnvalue (`KismetMathLibrary.MakeVector` (`KismetMathLibrary.FClamp` _returnvalue_x 0.0 (* (`/Game/Road_Creator_Pro/Blueprints/BP_Road_Creator.Length, m` (`local.Current Road`)) 100.0))))))
        (set `local.Current Min Distance` (`KismetMathLibrary.Vector_Distance` (`self.K2_GetActorLocation`) _output_get_3))))
    (if (< (`local.Current Min Distance`) (`local.Min Distance`))
      (set `local.Min Distance` (`local.Current Min Distance`))
      (set `self.Distance on Spline` _distance_on_spline)
      (bind _output_get_4 (set `self.Road` (`local.Current Road`)))
      (set `self.Spline` (`/Game/Road_Creator_Pro/Blueprints/BP_Road_Creator.Input Spline` _output_get_4))
      (set `self.Closest Location` (`local.Current Closest Location`)))))

(fn `Search Closest Point On Spline`
  (params (Spline :type "SplineComponent Object Reference") (Location :type "Vector Structure") (`Segment Length` :type "Float (double-precision)" :default 300.0))
  (returns (`Distance on Spline` :type "Float (double-precision)") (`Closest Location` :type "Vector Structure"))
  (locals (MinDistance :type "Float (double-precision)") (`Positition Index` :type Integer) (SegmentLength :type "Float (double-precision)" :default 100.0) (`Location local` :type "Vector Structure") (`Spline local` :type "SplineComponent Object Reference") (`Distance (Key before)` :type "Float (single-precision)" :default 0.0) (`Distance (Key after)` :type "Float (single-precision)" :default 0.0) (`Loops Number` :type Integer :default 0) (`Temp Location` :type "Vector Structure" :default (0.0 0.0 0.0)) (`Output Location` :type "Vector Structure"))
  (bind _spline_local (`local.Spline local`))
  (bind _returnvalue (`KismetMathLibrary.FFloor` (`SplineComponent.FindInputKeyClosestToWorldLocation` (`local.Spline local`) (`local.Location local`))))
  ; Downloaded from t.me/FABUE5AssetsFree
  ; Best environments, models, plugins, animations, VFX, SFX, templates for Unreal Engine
  (set `local.Spline local` Spline)
  (set `local.Location local` Location)
  (set `local.SegmentLength` `Segment Length`)
  (set `local.MinDistance` 10000.0)
  (if (not false)
    ;;[1 1 1] Search through all Spline
    (set `local.Distance (Key before)` (`SplineComponent.GetDistanceAlongSplineAtSplinePoint` _spline_local _returnvalue))
    (set `local.Distance (Key after)` (`SplineComponent.GetDistanceAlongSplineAtSplinePoint` _spline_local (+ _returnvalue 1)))
    (set `local.Loops Number` (`KismetMathLibrary.FCeil` (`KismetMathLibrary.Abs` (/ (- (`local.Distance (Key before)`) (`local.Distance (Key after)`)) (`local.SegmentLength`)))))
    (for _index (range (+ (`local.Loops Number`) 1))
      (bind _output_get (set `local.Temp Location` (`SplineComponent.GetLocationAtDistanceAlongSpline` (`local.Spline local`) (+ (`local.Distance (Key before)`) (* _index (`local.SegmentLength`))) "World")))
      (bind _returnvalue_2 (`KismetMathLibrary.VSize` (- (`local.Location local`) _output_get)))
      (if (< _returnvalue_2 (`local.MinDistance`))
        (set `local.MinDistance` _returnvalue_2)
        (set `local.Positition Index` _index)
        (set `local.Output Location` (`local.Temp Location`))))
    (return (+ (`local.Distance (Key before)`) (* (`local.Positition Index`) (`local.SegmentLength`))) (`local.Output Location`))))

(fn `UserConstructionScript`
  (bind _mesh (`self.Mesh`))
  (bind _road (`self.Road`))
  (bind (_mesh_rotation_roll _mesh_rotation_pitch _mesh_rotation_yaw) (`KismetMathLibrary.BreakRotator` (`self.Mesh Rotation`)))
  (bind _asphalt_material (`self.Asphalt Material`))
  (bind _spline (`self.Spline`))
  (bind _spline_2 (`self.Spline`))
  (bind _distance_on_spline (`self.Distance on Spline`))
  (bind _junction_halfwidth (`self.Junction HalfWIdth`))
  (bind _returnvalue (`self.K2_GetActorRotation` (`self.Road`)))
  (bind _returnvalue_2 (`KismetMathLibrary.SelectFloat` 1.0 -1.0 (`self.On Right Side`)))
  (bind _returnvalue_3 (- _distance_on_spline _junction_halfwidth))
  (bind _returnvalue_4 (+ _distance_on_spline _junction_halfwidth))
  (bind (_road_settings_roadmesh _road_settings_guardrailallowed _road_settings_guardrailsideoffset _road_settings_sidewalkfenceallowed _road_settings_sidewalkfencesideoffset _road_settings_reflectorpolesallowed _road_settings_reflectorpolessideoffset _road_settings_sidewalkallowed _road_settings_sidewalksideoffset _road_settings_landscapedeformwidth _road_settings_bridgemesh _road_settings_lamppostsoffset _road_settings_lamppostsheight _road_settings_bridgesupportscaleoffset _road_settings_isbridge _road_settings_concretebarrieroffset) (break `/Game/Road_Creator_Pro/Blueprints/Helpers/Road_Type_Settings` (`/Game/Road_Creator_Pro/Blueprints/BP_Road_Creator.Road Settings` _road)))
  (bind _returnvalue_5 (`|EnumEquality` (`/Game/Road_Creator_Pro/Blueprints/BP_Road_Creator.Road Type` _road) "NewEnumerator12"))
  (bind _returnvalue_6 (/ (* (`/Game/Road_Creator_Pro/Blueprints/BP_Road_Creator.Wider gap at the End` (`self.Road`)) 100.0) (`SplineComponent.GetSplineLength` (`self.Spline`))))
  (bind _returnvalue_7 (+ (`SplineComponent.GetLocationAtDistanceAlongSpline` _spline _returnvalue_4 "World") (* (`SplineComponent.GetRightVectorAtDistanceAlongSpline` _spline _returnvalue_4 "World") (+ (`self.Side Offset`) (* _returnvalue_6 _returnvalue_4) (`self.Offset Lateral`)) _returnvalue_2)))
  (bind _returnvalue_8 (+ (`SplineComponent.GetLocationAtDistanceAlongSpline` _spline_2 _returnvalue_3 "World") (* (`SplineComponent.GetRightVectorAtDistanceAlongSpline` _spline_2 _returnvalue_3 "World") (+ (`self.Side Offset`) (* _returnvalue_6 _returnvalue_3) (`self.Offset Lateral`)) _returnvalue_2)))
  ;[1 1 1] Set Mesh
  (`StaticMeshComponent.SetStaticMesh` (`self.Junction Mesh`) _mesh)
  (set `self.Junction HalfWIdth` (.x (`.BoxExtent` (`KismetMathLibrary.BreakBoxSphereBounds` (`StaticMesh.GetBounds` _mesh)))))
  ;[1 1 1] Find Closest Road
  (`self.Find closest Road`)
  (`/Engine/EditorBlueprintResources/StandardMacros.IsValid` (`self.Road`)
    (:`Is Valid`
      (`|ExecutionSequence`
        (:`then_1`
          ;[1 1 1] Get Road Parameters
          (set `self.Road Uses Spline` (`/Game/Road_Creator_Pro/Blueprints/BP_Road_Creator.Use Spline` (`self.Road`)))
          (set `self.On Right Side` (> (`KismetMathLibrary.Dot_VectorVector` (- (`self.K2_GetActorLocation`) (`self.Closest Location`)) (select `bool` (`self.Road Uses Spline`) :`false` (`self.GetActorRightVector` (`self.Road`)) :`true` (`SplineComponent.GetRightVectorAtDistanceAlongSpline` (`self.Spline`) (`self.Distance on Spline`) "World"))) 0.0))
          (set `self.Side Offset` (+ (`KismetMathLibrary.SelectFloat` 0.0 (* (`/Game/Road_Creator_Pro/Blueprints/BP_Road_Creator.Road Width Multiplier` _road) (- _road_settings_concretebarrieroffset 60.0)) _returnvalue_5) (* (`/Game/Road_Creator_Pro/Blueprints/BP_Road_Creator.Two Roads Gap final` _road) (`/Game/Road_Creator_Pro/Blueprints/BP_Road_Creator.🔃 Two Roads` _road)) (`KismetMathLibrary.SelectFloat` -40.0 0.0 (`|EnumEquality` (`/Game/Road_Creator_Pro/Blueprints/BP_Road_Creator.Road Type` _road) "NewEnumerator7"))))
          (set `self.Wet` (`/Game/Road_Creator_Pro/Blueprints/BP_Road_Creator.Wet` _road))
          (if (not _returnvalue_5)
            (set `self.Asphalt Material` (`/Game/Road_Creator_Pro/Blueprints/BP_Road_Creator.Asphalt Material` _road))))
        (:`then_2`
          (`|ExecutionSequence`
            (:`then_0`
              (if (`self.Road Uses Spline`)
                ;[1 1 1] Position and Rotation (Spline Road)
                (set `self.Mesh Location` (+ (/ (+ _returnvalue_8 _returnvalue_7) 2.0) (`KismetMathLibrary.MakeVector` 0.0 0.0 (`self.Offset Vertical`))))
                (if (`self.On Right Side`)
                  (set `self.Mesh Rotation` (`KismetMathLibrary.FindLookAtRotation` _returnvalue_7 _returnvalue_8))
                  (else
                    (set `self.Mesh Rotation` (`KismetMathLibrary.FindLookAtRotation` _returnvalue_8 _returnvalue_7))))
                (else
                  ;[1 1 1] Position and Rotation (Straight Road)
                  (set `self.Mesh Location` (+ (`self.Closest Location`) (* (`self.GetActorRightVector` (`self.Road`)) (+ (`self.Side Offset`) (`self.Offset Lateral`)) (`KismetMathLibrary.SelectFloat` 1.0 -1.0 (`self.On Right Side`))) (`KismetMathLibrary.MakeVector` 0.0 0.0 (`self.Offset Vertical`))))
                  (if (`self.On Right Side`)
                    (set `self.Mesh Rotation` (`KismetMathLibrary.MakeRotationFromAxes` (* (`KismetMathLibrary.GetForwardVector` _returnvalue) -1.0) (* (`KismetMathLibrary.GetRightVector` _returnvalue) -1.0) (`KismetMathLibrary.GetUpVector` _returnvalue)))
                    (else
                      (set `self.Mesh Rotation` _returnvalue))))))
            (:`then_1`
              ;[1 1 1] Pitch and Scale
              (set `self.Mesh Scale` (`KismetMathLibrary.MakeVector` (* (`self.Width`) (`KismetMathLibrary.SelectFloat` -1.0 1.0 (`self.Mirror Longitudinal`))) (`KismetMathLibrary.SelectFloat` -1.0 1.0 (`self.Mirror Lateral`)) 1.0))
              (set `self.Mesh Rotation` (`KismetMathLibrary.MakeRotator` (+ _mesh_rotation_roll (`self.Pitch`)) _mesh_rotation_pitch _mesh_rotation_yaw)))
            (:`then_2`
              ;[1 1 1] Adjust Mesh
              (`SceneComponent.K2_SetWorldTransform` (`self.Junction Mesh`) (`KismetMathLibrary.MakeTransform` (`self.Mesh Location`) (`self.Mesh Rotation`) (`self.Mesh Scale`)) false true)
              (`|ExecutionSequence`
                (:`then_0`
                  (`/Engine/EditorBlueprintResources/StandardMacros.IsValid` _asphalt_material
                    (:`Is Valid`
                      (`PrimitiveComponent.SetMaterial` (`self.Junction Mesh`) 0 _asphalt_material))))
                (:`then_1`
                  (`MeshComponent.SetScalarParameterValueOnMaterials` (`self.Junction Mesh`) "Wet" (`self.Wet`)))))))))))