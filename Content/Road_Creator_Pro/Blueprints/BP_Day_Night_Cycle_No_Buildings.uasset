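; Day/night cycle actor that advances time of day, rotates the level's directional light by latitude and season, and toggles sun and optional moon light visibility.
; Tick interval scales with day length, and sun rotation updates at half rate once below the horizon.
; A timer switches BPI_Light_Control actors at dusk and dawn, staggered in shuffled order.
; A timeline supports fast time skips, and the construction script provides an editor preview.
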(event Custom|Update_Actors_Event
  (CallFunction|UpdateActors false))

(event Custom|Switch%20Lights%20on%20Actors%20with%20Lights%20Interface
  (params (First%20Time :type Boolean))
  ;[1 1 1] Switch Lights on Actors with Lights Interface
  ;;[1 1 1] Prepare for Loop (in random order)
  (Utilities|Array|Shuffle (Variables|Default|GetActors%20with%20Light%20Interface))
  (Variables|Default|SetIndex 0)
  (if (or First%20Time (Variables|Default|GetTime%20Skipping)) :!label _label
    _
    (else
      ;;[1 1 1] Gradually switch all actors during some time period
      (Utilities|FlowControl|Delay (/ (/ (* (Variables|Default|GetDay%20Duration%20%28minutes%29) 0.6) (Utilities|Array|Length (Variables|Default|GetActors%20with%20Light%20Interface))) (Variables|Default|GetActors%20with%20Lights%20Interface%20Switch%20Speed)))))
  (Class|BPILightControl|SwitchLights(Message) (Utilities|Array|Get(acopy) (Variables|Default|GetActors%20with%20Light%20Interface) (Variables|Default|GetIndex)) (Variables|Default|GetActors%20with%20Light%20Interface%20are%20ON))
  ;;[1 1 1] Loop
  (bind _result (Math|Integer|IncrementInt (Variables|Default|GetIndex))
    (:%20%20
      (if (not (> _result (Utilities|Array|LastIndex (Variables|Default|GetActors%20with%20Light%20Interface))))
        (goto _label)))))

(event Custom|Fast%20Skip%20Time
  (params (Hours%20delta :type Float%20%28double-precision%29) (Skip%20Time%20seconds :type Float%20%28double-precision%29))
  ;[1 1 1] Fast Skip Time
  (if (not (Variables|Default|GetTime%20Skipping))
    (Variables|Default|SetTime%20Before%20Skip (Variables|Default|GetTime_Of_Day))
    (Variables|Default|SetTime%20Skipping true)
    (Actor|Tick|SetActorTickInterval 0.0)
    (Components|Timeline|SetPlayRate (Variables|Default|GetTimeline) (/ 1.0 Skip%20Time%20seconds))
    (bind _progress (Timeline|Timeline PlayFromStart)
      (:Update
        (Variables|Default|SetTime_Of_Day (+ (* _progress Hours%20delta) (Variables|Default|GetTime%20Before%20Skip)))
        (CallFunction|UpdateActors false))
      (:Finished
        (Variables|Default|SetTime%20Skipping false)
        (Actor|Tick|SetActorTickInterval (Variables|Default|GetTick%20Interval))))))

(event EventBeginPlay
  (if (Variables|Default|GetEnabled%20in%20Game)
    (Variables|Default|SetEnabled%20in%20Game false)
    (Utilities|FlowControl|DelayUntilNextTick)
    (bind _returnvalue (Actor|GetActorOfClass "/Script/Engine.DirectionalLight"))
    (Utilities|IsValid _returnvalue
      (:Is%20Valid
        (bind _output_get (Variables|Default|SetSun%20Light _returnvalue))
        (Variables|Default|SetSun%20ON (Rendering|IsVisible (Variables|/Script/Engine.Light|GetLightComponent _output_get)))
        (Variables|Default|SetEnabled%20in%20Game true)
        (if (Variables|Default|GetUpdate%20Actors)
          (Utilities|FlowControl|DelayUntilNextTick)
          (Utilities|FlowControl|DelayUntilNextTick)
          (CallFunction|GetAllActorswithInterface)
          (CallFunction|UpdateActors true)
          (Utilities|FlowControl|DelayUntilNextTick)
          (Utilities|FlowControl|DelayUntilNextTick)
          (Utilities|Time|SetTimerbyEvent (delegate Custom|Update_Actors_Event) (* (Variables|Default|GetDay%20Duration%20%28minutes%29) 0.08) true)))
      (:Is%20Not%20Valid
        (Variables|Default|SetEnabled%20in%20Game false)))))

(event EventTick
  (params (DeltaSeconds :type Float%20%28single-precision%29))
  (if (Variables|Default|GetEnabled%20in%20Game)
    (Utilities|FlowControl|Sequence
      (:then_0
        ;[1 1 1] Cycle Time of Day
        (bind _output_get (Variables|Default|SetTime_Of_Day (+ (Variables|Default|GetTime_Of_Day) (* DeltaSeconds (/ 0.4 (Variables|Default|GetDay%20Duration%20%28minutes%29))))))
        (if (>= _output_get 24.0)
          (Variables|Default|SetTime_Of_Day 0.0)))
      (:then_1
        (bind _isa (Utilities|FlowControl|FlipFlop)
          (:A
            _)
          (:B
            _))
        (CallFunction|RotateSun _isa)))))

(fn ConstructionScript
  (bind _moon_light (Variables|Default|GetMoon_Light))
  (Utilities|FlowControl|Sequence
    (:then_0
      (if (Variables|Default|GetEnabled%20in%20Editor)
        (bind _returnvalue (Actor|GetActorOfClass "/Script/Engine.DirectionalLight"))
        (Utilities|IsValid _returnvalue
          (:Is%20Valid
            (bind _output_get (Variables|Default|SetSun%20Light _returnvalue))
            (Variables|Default|SetSun%20ON (Rendering|IsVisible (Variables|/Script/Engine.Light|GetLightComponent _output_get)))
            (CallFunction|RotateSun false))
          (:Is%20Not%20Valid
            _))
        (if (Variables|Default|GetUpdate%20Actors)
          (CallFunction|GetAllActorswithInterface)
          (CallFunction|UpdateActors true)
          (Utilities|Array|Clear (Variables|Default|GetActors%20with%20Light%20Interface)))))
    (:then_1
      (if (Variables|Default|GetMoon)
        (Rendering|Components|Light|SetIntensity _moon_light (Variables|Default|GetMoon%20Brightness))
        (else
          (Components|DestroyComponent _moon_light))))
    (:then_2
      ;[1 1 1] Set Tick Interval
      (bind _output_get_2 (Variables|Default|SetTick%20Interval (* (/ (Variables|Default|GetDay%20Duration%20%28minutes%29) 8e+01) (Variables|Default|GetSun%20Update%20Interval))))
      (Actor|Tick|SetActorTickInterval _output_get_2))))

(fn RotateSun
  (params (FlipFlop :type Boolean))
  (bind _moon_light (Variables|Default|GetMoon_Light))
  (bind _sun_light (Variables|Default|GetSun%20Light))
  (bind _lightcomponent (Variables|/Script/Engine.Light|GetLightComponent _sun_light))
  ;[1 1 1] Calculate Sun Pitch
  (LocalVariables|SetSun%20Pitch (|(((90-Lat)*(cos(((Time/12)*3.141500))))-SeasonalTilt) (Variables|Default|GetTime_Of_Day) (Variables|Default|GetSeason%20Tilt) (Math|Float|Absolute(Float) (Variables|Default|GetLatitude))))
  (Utilities|FlowControl|Sequence
    (:then_1
      (if (< (LocalVariables|GetSun%20Pitch) 8.0)
        (if (not (Variables|Default|GetSun%20ON))
          (Rendering|SetVisibility _lightcomponent true false)
          (Variables|Default|SetSun%20ON true))
        (elif (Variables|Default|GetSun%20ON)
          (Rendering|SetVisibility _lightcomponent false false)
          (Variables|Default|SetSun%20ON false))))
    (:then_2
      (if (Variables|Default|GetMoon)
        (if (< (LocalVariables|GetSun%20Pitch) 0.2)
          (if (Variables|Default|GetMoon%20ON)
            (Rendering|SetVisibility _moon_light false false)
            (Variables|Default|SetMoon%20ON false))
          (elif (not (Variables|Default|GetMoon%20ON))
            (Rendering|SetVisibility _moon_light true false)
            (Variables|Default|SetMoon%20ON true)))))
    (:then_3
      ;[1 1 1] Rotate Sun
      (if (Variables|Default|GetSun%20ON)
        (if (< (LocalVariables|GetSun%20Pitch) 3.0)
          (Transformation|SetWorldRotation (Variables|/Script/Engine.Light|GetLightComponent (Variables|Default|GetSun%20Light)) (Math|Rotator|MakeRotator 0.0 (LocalVariables|GetSun%20Pitch) (+ (* (Math|Float|Sign(Float) (+ (Variables|Default|GetLatitude) 0.01)) (|((Time*15)+90) (Variables|Default|GetTime_Of_Day))) (.yaw (Transformation|GetActorRotation)))) false false :!label _label)
          (elif (not FlipFlop)
            (goto _label)))))))

(fn UpdateActors
  (params (First%20time :type Boolean))
  (bind _time_of_day (Variables|Default|GetTime_Of_Day))
  (Variables|Default|SetTime_Of_Day_Tilt_Corrected (+ (* (Math|Trig|Sin(Degrees) (* _time_of_day 15.0)) (Variables|Default|GetSeason%20Tilt) 0.13) _time_of_day))
  ;[1 1 1] Update actors with Light Interface
  (if (Utilities|Array|IsNotEmpty (Variables|Default|GetActors%20with%20Light%20Interface))
    (if First%20time
      (Variables|Default|SetActors%20with%20Light%20Interface%20are%20ON (not (Math|Float|InRange(Float) (Variables|Default|GetTime_Of_Day_Tilt_Corrected) 6.1 17.6)) :!label _label)
      (CallFunction|SwitchLightsonActorswithLightsInterface First%20time)
      (elif (!= (not (Math|Float|InRange(Float) (Variables|Default|GetTime_Of_Day_Tilt_Corrected) 6.1 17.6)) (Variables|Default|GetActors%20with%20Light%20Interface%20are%20ON))
        (goto _label)))))

(fn GetAllActorswithInterface
  (bind _outactors (Actor|GetAllActorswithInterface "/Game/Road_Creator_Pro/Blueprints/Helpers/BPI_Light_Control.BPI_Light_Control_C"))
  (Variables|Default|SetActors%20with%20Light%20Interface _outactors))