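; Road expansion joint actor from Road Creator Pro that shows a decal and plays a bump sound when an actor crosses it.
; The construction script scales the trigger box and decal from Length and Width, adjusting decal material tiling to the length.
; On overlap, the other actor's speed in km/h drives the attenuated sound's volume and pitch.
; A DoOnce with a short delayed reset limits rapid retriggering.
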(event `self.Box.OnComponentBeginOverlap`
  (params (OverlappedComponent :type "PrimitiveComponent Object Reference") (OtherActor :type "Actor Object Reference") (OtherComp :type "PrimitiveComponent Object Reference") (OtherBodyIndex :type Integer) (bFromSweep :type Boolean) (SweepResult :type "HitResult Structure (by ref)"))
  (`/Engine/EditorBlueprintResources/StandardMacros.DoOnce` false :!label _label
    (:`Completed`
      (`|ExecutionSequence`
        (:`then_0`
          ;[1 1 1] Get Vehicle speed
          (bind _output_get (set `self.Vehicle Speed km/h` (* (`KismetMathLibrary.Abs` (`KismetMathLibrary.VSize` (`self.GetVelocity` OtherActor))) 0.036)))
          ;[1 1 1] Play Sound
          (`GameplayStatics.PlaySoundAtLocation` "/Game/Road_Creator_Pro/Sound/SC_Expansion_Joint.SC_Expansion_Joint" (`self.K2_GetActorLocation`) (struct) (* (`KismetMathLibrary.MapRangeClamped` _output_get 10.0 90.0 0.0 1.0) (`self.Volume Multiplier`)) (`KismetMathLibrary.MapRangeClamped` _output_get 20.0 100.0 0.6 1.2) 0.0 "/Game/Road_Creator_Pro/Sound/NewSoundAttenuation.NewSoundAttenuation" null null null))
        (:`then_1`
          (`KismetSystemLibrary.Delay` 0.05)
          (goto _label :!via `Reset`))))))

(fn `UserConstructionScript`
  (bind _decal (`self.Decal`))
  (bind _returnvalue (/ (`self.Length`) 8.0))
  (set `self.❓Hover for Help ` false)
  (`SceneComponent.SetRelativeScale3D` (`self.Box`) (`KismetMathLibrary.MakeVector` 1.0 _returnvalue 1.0))
  (`SceneComponent.SetRelativeScale3D` _decal (`KismetMathLibrary.MakeVector` 1.0 (/ (`self.Width`) 40.0) _returnvalue))
  (bind _returnvalue_2 (`DecalComponent.CreateDynamicMaterialInstance` _decal))
  (`MaterialInstanceDynamic.SetScalarParameterValue` _returnvalue_2 "U Tiling" (* _returnvalue 15.0))
  (if (== (`self.Volume Multiplier`) 0.0)
    _))