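; Road Creator Pro decal actor, named for leaks and graffiti, that projects a configurable texture and is set up entirely in the Construction Script.
; When a texture is valid, it creates a dynamic material instance and feeds in color, opacity and the texture.
; It shrinks the decal's relative Y or Z scale to match the Texture2D's aspect ratio, and always applies the sort order.
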(fn `UserConstructionScript`
  (bind _decal_texture (`self.Decal Texture`))
  (bind _decal (`self.Decal`))
  (`|ExecutionSequence`
    (:`then_0`
      (`/Engine/EditorBlueprintResources/StandardMacros.IsValid` _decal_texture
        (:`Is Valid`
          (`|ExecutionSequence`
            (:`then_1`
              (bind _returnvalue (`DecalComponent.CreateDynamicMaterialInstance` (`self.Decal`)))
              (`MaterialInstanceDynamic.SetVectorParameterValue` _returnvalue "Color" (`KismetMathLibrary.Conv_ColorToLinearColor` (`self.Color`)))
              (`MaterialInstanceDynamic.SetScalarParameterValue` _returnvalue "Opacity" (`self.Opacity`)))
            (:`then_2`
              (`MaterialInstanceDynamic.SetTextureParameterValue` _returnvalue "Texture" _decal_texture)
              (bind _astexture_2d (cast `Texture2D` _decal_texture))
              (`|ExecutionSequence`
                (:`then_0`
                  (bind _returnvalue_2 (`Texture2D.Blueprint_GetSizeX` _astexture_2d))
                  (bind _returnvalue_3 (`Texture2D.Blueprint_GetSizeY` _astexture_2d))
                  (if (> _returnvalue_2 _returnvalue_3)
                    (`SceneComponent.SetRelativeScale3D` _decal (`KismetMathLibrary.MakeVector` 1.0 (/ _returnvalue_3 _returnvalue_2) 1.0))))
                (:`then_1`
                  (if (< _returnvalue_2 _returnvalue_3)
                    (`SceneComponent.SetRelativeScale3D` _decal (`KismetMathLibrary.MakeVector` 1.0 1.0 (/ _returnvalue_2 _returnvalue_3)))))))))))
    (:`then_1`
      (`DecalComponent.SetSortOrder` (`self.Decal`) (`self.Sort Order`)))))