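; Road marking decal actor that draws either a solid or dashed line, or a textured marking, from its exposed settings.
; The construction script picks a material from the line, dash and retroreflective flags, then sets sort order and dynamic parameters for color, cracks, dashes or texture.
; Lines scale by length and width, while textures keep their aspect ratio with optional mirroring, recalculated at BeginPlay if Scale is still one.
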(event `self.ReceiveBeginPlay`
  (if (`self.Line`)
    _
    (elif (== (`self.Scale`) (1.0 1.0 1.0))
      (`self.Set Decal Proportions`))))

(fn `Set Decal Proportions`
  (bind _size_normalized (`self.Size normalized`))
  (bind _astexture_2d (cast `Texture2D` (`self.Decal Texture`)))
  (`|ExecutionSequence`
    (:`then_0`
      (bind _returnvalue (`Texture2D.Blueprint_GetSizeX` _astexture_2d))
      (bind _returnvalue_2 (`Texture2D.Blueprint_GetSizeY` _astexture_2d))
      (if (> _returnvalue _returnvalue_2)
        (set `self.Scale` (`KismetMathLibrary.MakeVector` 1.0 (/ _returnvalue_2 _returnvalue) 1.0))))
    (:`then_1`
      (if (< _returnvalue _returnvalue_2)
        (set `self.Scale` (`KismetMathLibrary.MakeVector` 1.0 1.0 (/ _returnvalue _returnvalue_2)))))
    (:`then_2`
      (`SceneComponent.SetRelativeScale3D` (`self.Decal`) (* (`self.Scale`) (`KismetMathLibrary.MakeVector` 1.0 _size_normalized _size_normalized) (`KismetMathLibrary.MakeVector` (/ (`self.Height`) 10.0) 1.0 (`KismetMathLibrary.SelectFloat` -1.0 1.0 (`self.Mirror`))))))))

(fn `UserConstructionScript`
  (bind _line (`self.Line`))
  (bind _dashed_line (`self.Dashed Line`))
  (bind _decal_material (`self.Decal Material`))
  (bind (_returnvalue_r _returnvalue_g _returnvalue_b _returnvalue_a) (break `LinearColor` (`KismetMathLibrary.Conv_ColorToLinearColor` (`self.Color`))))
  (`|ExecutionSequence`
    (:`then_0`
      (set `self.Size normalized` (/ (`self.Size, m`) 5.0)))
    (:`then_1`
      ;[1 1 1] Set Decal Material
      (`DecalComponent.SetDecalMaterial` (`self.Decal`) (select `bool` (`self.Retro-Reflective`) :`false` (select `bool` _line :`false` "/Game/Road_Creator_Pro/Materials/Markings/MI_Markings_Decal.MI_Markings_Decal" :`true` (select `bool` _dashed_line :`false` "/Game/Road_Creator_Pro/Materials/Markings/MI_Markings_Decal_NoTexture_RR.MI_Markings_Decal_NoTexture_RR" :`true` "/Game/Road_Creator_Pro/Materials/Markings/MI_Markings_Decal_NoTexture_Dashed_RR.MI_Markings_Decal_NoTexture_Dashed_RR" :!type "MaterialInterface Object Reference")) :`true` (select `bool` _line :`false` "/Game/Road_Creator_Pro/Materials/Markings/MI_Markings_Decal_RR.MI_Markings_Decal_RR" :`true` (select `bool` _dashed_line :`false` "/Game/Road_Creator_Pro/Materials/Markings/MI_Markings_Decal_NoTexture.MI_Markings_Decal_NoTexture" :`true` "/Game/Road_Creator_Pro/Materials/Markings/MI_Markings_Decal_NoTexture_Dashed.MI_Markings_Decal_NoTexture_Dashed" :!type "MaterialInterface Object Reference")))))
    (:`then_2`
      (if (`self.Line`)
        (`SceneComponent.SetRelativeScale3D` (`self.Decal`) (`KismetMathLibrary.MakeVector` (/ (`self.Height`) 10.0) (`self.Size normalized`) (/ (`self.Line Width, cm`) 500.0)))
        (bind _returnvalue (`DecalComponent.CreateDynamicMaterialInstance` (`self.Decal`) :!label _label))
        ;[1 1 1] Set Color
        (bind _output_get (set `self.Decal Material` _returnvalue))
        (`MaterialInstanceDynamic.SetVectorParameterValue` _output_get "Color" (make `LinearColor` _returnvalue_r _returnvalue_g _returnvalue_b (* _returnvalue_a (`self.Opacity`))))
        (`MaterialInstanceDynamic.SetScalarParameterValue` _output_get "Cracks Amount" (`self.Cracks Amount`))
        ;[1 1 1] Dashed Line setup
        (if (`self.Dashed Line`)
          (`MaterialInstanceDynamic.SetScalarParameterValue` _decal_material "Number of Dashes" (/ (`self.Size, m`) (`self.Dashed Period, m`)))
          (`MaterialInstanceDynamic.SetScalarParameterValue` _decal_material "Gap Width" (`self.Dashed Gap`)))
        (else
          (`/Engine/EditorBlueprintResources/StandardMacros.IsValid` (`self.Decal Texture`)
            (:`Is Valid`
              (`|ExecutionSequence`
                (:`then_0`
                  (goto _label))
                (:`then_1`
                  (`MaterialInstanceDynamic.SetTextureParameterValue` (`self.Decal Material`) "Texture" (`self.Decal Texture`))
                  (`self.Set Decal Proportions`))))))))
    (:`then_3`
      (`DecalComponent.SetSortOrder` (`self.Decal`) (`self.Sort Order`)))))