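; Parent Blueprint for barrier rows in Road Creator Pro that builds poles, optional chains and panels as instanced static meshes in the Construction Script.
; It lays them along the spline as straight point-to-point segments or evenly by distance, or in a straight X-axis row with the spline destroyed.
; Chains and panels scale in X to span the spacing, KeepVertical removes pitch, and components for unused parts are destroyed.
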(fn `UserConstructionScript`
  (locals (`Current num of Segments` :type Integer :default 0) (`Current X Scale` :type "Float (double-precision)") (`Current Rotation` :type "Rotator Structure" :default (struct)))
  (bind _pole_material (`self.Pole Material`))
  (bind _chain_material (`self.Chain Material`))
  (bind _instancedstaticmesh_panel (`self.InstancedStaticMesh_Panel`))
  (bind _panel_material (`self.Panel Material`))
  (bind _spacing (`self.Spacing`))
  (bind _spline (`self.Spline`))
  (bind _spacing_calculated (`self.Spacing calculated`))
  (bind _spline_2 (`self.Spline`))
  (bind _spacing_calculated_2 (`self.Spacing calculated`))
  (bind _spacing_2 (`self.Spacing`))
  (bind _spline_3 (`self.Spline`))
  (bind _spline_4 (`self.Spline`))
  (bind _instancedstaticmesh_pole (`self.InstancedStaticMesh_Pole`))
  (bind (_current_rotation_roll _current_rotation_pitch _current_rotation_yaw) (`KismetMathLibrary.BreakRotator` (`local.Current Rotation`)))
  (bind _spline_5 (`self.Spline`))
  (bind _panel_mesh (`self.Panel Mesh`))
  (bind _returnvalue (`SplineComponent.GetSplineLength` (`self.Spline`)))
  (bind _returnvalue_2 (`KismetMathLibrary.SelectRotator` (`KismetMathLibrary.MakeRotator` 0.0 0.0 _current_rotation_yaw) (`local.Current Rotation`) (`self.Keep Vertical`)))
  (bind _returnvalue_3 (`KismetMathLibrary.FCeil` (/ _returnvalue (`self.Spacing`))))
  (bind _returnvalue_4 (`KismetMathLibrary.MakeRotator` (.roll _returnvalue_2) (.pitch _returnvalue_2) (+ (`self.Pole Rotation`) (.yaw _returnvalue_2))))
  (`|ExecutionSequence`
    (:`then_1`
      ;[1 1 1] Set Pole Mesh
      (`/Engine/EditorBlueprintResources/StandardMacros.IsValid` (`self.Pole Mesh`)
        (:`Is Valid`
          (`StaticMeshComponent.SetStaticMesh` _instancedstaticmesh_pole (`self.Pole Mesh`))
          (`/Engine/EditorBlueprintResources/StandardMacros.IsValid` _pole_material
            (:`Is Valid`
              (`PrimitiveComponent.SetMaterial` _instancedstaticmesh_pole 0 _pole_material))
            (:`Is Not Valid`)))
        (:`Is Not Valid`
          (`ActorComponent.K2_DestroyComponent` (`self.InstancedStaticMesh_Pole`)))))
    (:`then_2`
      ;[1 1 1] Set Panel Mesh
      (`/Engine/EditorBlueprintResources/StandardMacros.IsValid` _panel_mesh
        (:`Is Valid`
          (`StaticMeshComponent.SetStaticMesh` _instancedstaticmesh_panel _panel_mesh)
          (`/Engine/EditorBlueprintResources/StandardMacros.IsValid` _panel_material
            (:`Is Valid`
              (`PrimitiveComponent.SetMaterial` _instancedstaticmesh_panel 0 _panel_material))
            (:`Is Not Valid`)))
        (:`Is Not Valid`
          (`ActorComponent.K2_DestroyComponent` (`self.InstancedStaticMesh_Panel`)))))
    (:`then_3`
      ;[1 1 1] Set Chain
      (if (`self.Chain`)
        (`/Engine/EditorBlueprintResources/StandardMacros.IsValid` _chain_material
          (:`Is Valid`
            (`PrimitiveComponent.SetMaterial` (`self.InstancedStaticMesh_Chain`) 0 _chain_material))
          (:`Is Not Valid`))
        (else
          (`ActorComponent.K2_DestroyComponent` (`self.InstancedStaticMesh_Chain`)))))
    (:`then_5`
      (if (and (`self.Use Spline`) (`self.Straight Lines Spline`))
        ;[1 1 1] Straight Lines Spline
        (for _index (range (+ (- (`SplineComponent.GetNumberOfSplinePoints` (`self.Spline`)) 2) 1))
          (`|ExecutionSequence`
            (:`then_1`
              (bind _returnvalue_5 (`SplineComponent.GetLocationAtSplinePoint` _spline_4 _index "Local"))
              (bind _returnvalue_6 (`SplineComponent.GetLocationAtSplinePoint` _spline_4 (+ _index 1) "Local"))
              (bind _returnvalue_7 (`KismetMathLibrary.VSize` (- _returnvalue_5 _returnvalue_6)))
              (bind _output_get (set `local.Current num of Segments` (`KismetMathLibrary.FCeil` (/ _returnvalue_7 (`self.Spacing`)))))
              (set `local.Current X Scale` (/ _returnvalue_7 (* _output_get (`self.Spacing`))))
              (set `local.Current Rotation` (`KismetMathLibrary.FindLookAtRotation` _returnvalue_5 _returnvalue_6))
              (for _index_2 (range _output_get)
                (`|ExecutionSequence`
                  (:`then_0`
                    (`/Engine/EditorBlueprintResources/StandardMacros.IsValid` (`self.Pole Mesh`)
                      (:`Is Valid`
                        (bind _returnvalue_8 (`KismetMathLibrary.VLerp` _returnvalue_5 _returnvalue_6 (/ _index_2 (`local.Current num of Segments`))))
                        (`InstancedStaticMeshComponent.AddInstance` (`self.InstancedStaticMesh_Pole`) (`KismetMathLibrary.MakeTransform` (`KismetMathLibrary.SelectVector` (+ (`KismetMathLibrary.GreaterGreater_VectorRotator` (`KismetMathLibrary.MakeVector` (.x (`.BoxExtent` (`KismetMathLibrary.BreakBoxSphereBounds` (`StaticMesh.GetBounds` (`self.Pole Mesh`)))))) _returnvalue_4) _returnvalue_8) _returnvalue_8 (`self.Pivot at Center of Pole Mesh`)) _returnvalue_4) false))))
                  (:`then_1`
                    (if (`self.Chain`)
                      (`InstancedStaticMeshComponent.AddInstance` (`self.InstancedStaticMesh_Chain`) (`KismetMathLibrary.MakeTransform` _returnvalue_8 _returnvalue_2 (`KismetMathLibrary.MakeVector` (`local.Current X Scale`) 1.0 1.0)) false)))
                  (:`then_2`
                    (`/Engine/EditorBlueprintResources/StandardMacros.IsValid` (`self.Panel Mesh`)
                      (:`Is Valid`
                        (`InstancedStaticMeshComponent.AddInstance` (`self.InstancedStaticMesh_Panel`) (`KismetMathLibrary.MakeTransform` _returnvalue_8 _returnvalue_2 (`KismetMathLibrary.MakeVector` (`local.Current X Scale`) 1.0 1.0)) false)))))))))
        (if (not (`self.No last pole`))
          (`/Engine/EditorBlueprintResources/StandardMacros.IsValid` (`self.Pole Mesh`)
            (:`Is Valid`
              (`InstancedStaticMeshComponent.AddInstance` (`self.InstancedStaticMesh_Pole`) (`KismetMathLibrary.MakeTransform` (`SplineComponent.GetLocationAtSplinePoint` _spline_5 (- (`SplineComponent.GetNumberOfSplinePoints` _spline_5) 1) "Local") _returnvalue_4) false))))
        (else
          ;[1 1 1] Not Straight Lines Spline
          (`|ExecutionSequence`
            (:`then_0`
              (set `self.Direction Multiplier` (select `bool` (`self.Invert direction`) :`false` 1.0 :`true` -1.0)))
            (:`then_1`
              ;[1 1 1] Poles
              (if (`self.Use Spline`)
                (set `self.Poles` (+ _returnvalue_3 1))
                (set `self.Spacing calculated` (/ _returnvalue _returnvalue_3))
                (`/Engine/EditorBlueprintResources/StandardMacros.IsValid` (`self.Pole Mesh`)
                  (:`Is Valid`
                    (for _index_3 (range (`self.Poles`))
                      (bind _returnvalue_9 (* _index_3 (`self.Spacing calculated`)))
                      (bind (_returnvalue_roll _returnvalue_pitch _returnvalue_yaw) (`KismetMathLibrary.BreakRotator` (`KismetMathLibrary.MakeRotationFromAxes` (`SplineComponent.GetTangentAtDistanceAlongSpline` _spline _returnvalue_9 "Local") (`SplineComponent.GetRightVectorAtDistanceAlongSpline` _spline _returnvalue_9 "Local") (0.0 0.0 1.0))))
                      (`InstancedStaticMeshComponent.AddInstance` (`self.InstancedStaticMesh_Pole`) (`KismetMathLibrary.MakeTransform` (`SplineComponent.GetLocationAtDistanceAlongSpline` _spline _returnvalue_9 "Local") (`KismetMathLibrary.MakeRotator` 0.0 (`KismetMathLibrary.SelectFloat` 0.0 _returnvalue_pitch (`self.Keep Vertical`)) (+ (`self.Pole Rotation`) _returnvalue_yaw))) false))))
                (else
                  (`ActorComponent.K2_DestroyComponent` (`self.Spline`))
                  (`/Engine/EditorBlueprintResources/StandardMacros.IsValid` (`self.Pole Mesh`)
                    (:`Is Valid`
                      (for _index_4 (range (`self.Poles`))
                        (`InstancedStaticMeshComponent.AddInstance` (`self.InstancedStaticMesh_Pole`) (`KismetMathLibrary.MakeTransform` (`KismetMathLibrary.MakeVector` (* _index_4 (`self.Spacing`) (`self.Direction Multiplier`))) (`KismetMathLibrary.MakeRotator` 0.0 0.0 (`self.Pole Rotation`))) false)))))))
            (:`then_2`
              ;[1 1 1] Chain
              (if (`self.Chain`)
                (for _index_5 (range (+ (- (`self.Poles`) 2) 1))
                  (if (`self.Use Spline`)
                    (bind _returnvalue_10 (`SplineComponent.GetLocationAtDistanceAlongSpline` _spline_2 (* _index_5 _spacing_calculated_2) "Local"))
                    (bind (_returnvalue_roll_2 _returnvalue_pitch_2 _returnvalue_yaw_2) (`KismetMathLibrary.BreakRotator` (`KismetMathLibrary.FindLookAtRotation` _returnvalue_10 (`SplineComponent.GetLocationAtDistanceAlongSpline` _spline_2 (* (+ _index_5 1) _spacing_calculated_2) "Local"))))
                    (`InstancedStaticMeshComponent.AddInstance` (`self.InstancedStaticMesh_Chain`) (`KismetMathLibrary.MakeTransform` _returnvalue_10 (`KismetMathLibrary.MakeRotator` 0.0 (`KismetMathLibrary.SelectFloat` 0.0 _returnvalue_pitch_2 (`self.Keep Vertical`)) _returnvalue_yaw_2) (`KismetMathLibrary.MakeVector` (/ (- (`self.Spacing calculated`) 3.0) 100.0) 1.0 1.0)) false)
                    (else
                      (`InstancedStaticMeshComponent.AddInstance` (`self.InstancedStaticMesh_Chain`) (`KismetMathLibrary.MakeTransform` (`KismetMathLibrary.MakeVector` (* (+ (* _index_5 _spacing) 3.0) (`self.Direction Multiplier`))) (`KismetMathLibrary.MakeRotator` 0.0 0.0 (`KismetMathLibrary.SelectFloat` 180.0 0.0 (`self.Invert direction`))) (`KismetMathLibrary.MakeVector` (/ (- _spacing 6.0) 100.0) 1.0 1.0)) false))))))
            (:`then_3`
              ;[1 1 1] Panel
              (`/Engine/EditorBlueprintResources/StandardMacros.IsValid` (`self.Panel Mesh`)
                (:`Is Valid`
                  (for _index_6 (range (+ (- (`self.Poles`) 2) 1))
                    (if (`self.Use Spline`)
                      (bind _returnvalue_11 (`SplineComponent.GetLocationAtDistanceAlongSpline` _spline_3 (* _index_6 _spacing_calculated) "Local"))
                      (bind _returnvalue_12 (`SplineComponent.GetLocationAtDistanceAlongSpline` _spline_3 (* (+ _index_6 1) _spacing_calculated) "Local"))
                      (bind (_returnvalue_roll_3 _returnvalue_pitch_3 _returnvalue_yaw_3) (`KismetMathLibrary.BreakRotator` (`KismetMathLibrary.FindLookAtRotation` _returnvalue_11 _returnvalue_12)))
                      (`InstancedStaticMeshComponent.AddInstance` (`self.InstancedStaticMesh_Panel`) (`KismetMathLibrary.MakeTransform` _returnvalue_11 (`KismetMathLibrary.MakeRotator` 0.0 (`KismetMathLibrary.SelectFloat` 0.0 _returnvalue_pitch_3 (`self.Keep Vertical`)) _returnvalue_yaw_3) (`KismetMathLibrary.MakeVector` (/ (`KismetMathLibrary.VSize` (- _returnvalue_11 _returnvalue_12)) (.x (`.BoxExtent` (`KismetMathLibrary.BreakBoxSphereBounds` (`StaticMesh.GetBounds` (`self.Panel Mesh`))))) 2.02 (`self.Additional Panel Scale divider`)) 1.0 1.0)) false)
                      (else
                        (`InstancedStaticMeshComponent.AddInstance` (`self.InstancedStaticMesh_Panel`) (`KismetMathLibrary.MakeTransform` (`KismetMathLibrary.MakeVector` (* _index_6 _spacing_2 (`self.Direction Multiplier`))) (struct) (`KismetMathLibrary.MakeVector` (/ _spacing_2 (.x (`.BoxExtent` (`KismetMathLibrary.BreakBoxSphereBounds` (`StaticMesh.GetBounds` (`self.Panel Mesh`))))) 2.02) 1.0 1.0)) false)))))))))))))