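; Traffic light intersection actor that builds poles and lights in the construction script and cycles their signals at runtime.
; Construction spawns vehicle and pedestrian lights on pole sockets and user-set transforms, binding each to one of four approaches by relative yaw.
; A looping one-second timer steps the active way through timed green, yellow, red and optional red-yellow phases, supporting paired, single-way or mid-block operation.
; Each change updates emissive material parameters and optional spotlight colours.
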(event `self.ReceiveBeginPlay`
  (`KismetSystemLibrary.DelayUntilNextTick`)
  (`self.Update And Traffic Lights`)
  (`KismetSystemLibrary.K2_SetTimerDelegate` (delegate `main`) 1.0 true))

(event `main`
  (`self.Switch Intersection State`))

(fn `Add one Traffic Light mesh`
  (params (RelativeTransform :type "Transform Structure") (Pedestrian :type Boolean))
  (returns (Mesh :type "StaticMeshComponent Object Reference"))
  (locals (`Mesh local` :type "StaticMeshComponent Object Reference"))
  (bind _returnvalue (`AddComponent|NODE_AddStaticMeshComponent-3` :`RelativeTransform` (`KismetMathLibrary.MakeTransform` RelativeTransform_Location RelativeTransform_Rotation (* RelativeTransform_Scale (`self.🚦 Traffic Light Scale`)))))
  (bind _output_get (set `local.Mesh local` _returnvalue))
  (`|ExecutionSequence`
    (:`then_0`
      (`StaticMeshComponent.SetStaticMesh` (`local.Mesh local`) (select `bool` Pedestrian :`false` "/Game/Road_Creator_Pro/Meshes/Intersection/SM_Traffilc_Light.SM_Traffilc_Light" :`true` "/Game/Road_Creator_Pro/Meshes/Intersection/SM_Traffilc_Light_Pedestrian.SM_Traffilc_Light_Pedestrian" :!type "StaticMesh Object Reference")))
    (:`then_1`
      (`MeshComponent.SetVectorParameterValueOnMaterials` _output_get "Color" (`KismetMathLibrary.Conv_LinearColorToVector` (`KismetMathLibrary.Conv_ColorToLinearColor` (`self.🚦 Traffic Light Color`)))))
    (:`then_2`
      ;[1 1 1] Add SpotLights
      (if (`self.🚦 Add Spot Lights to Traffic Lights`)
        (bind _returnvalue_2 (`AddComponent|NODE_AddSpotLightComponent-0`))
        (`LightComponent.SetIntensity` _returnvalue_2 (* (`KismetMathLibrary.SelectFloat` 15.0 50.0 (`local.Pedestrian`)) (`self.🚦 SpotLight Intensity`) 0.1))
        (`SceneComponent.K2_AttachToComponent` _returnvalue_2 (`local.Mesh local`) "None" "KeepRelative" "KeepRelative" "KeepRelative" true)
        (`KismetArrayLibrary.Array_Add` (`self.Spot Lights`) _returnvalue_2)))
    (:`then_3`
      (`KismetArrayLibrary.Array_Add` (`self.Traffilc Light Array`) (make `/Game/Road_Creator_Pro/Blueprints/Helpers/Traffic_Lights` (`local.Mesh local`) 0 Pedestrian))
      (return (`local.Mesh local`)))))

(fn `Add Traffic LIghts And Bind Them`
  (locals (Binding :type Integer) (`Array Length` :type Integer))
  (bind _returnvalue (`self.GetActorScale3D`))
  (bind _traffilc_light_array (`self.Traffilc Light Array`))
  (bind _traffilc_light_array_2 (`self.Traffilc Light Array`))
  (bind _spot_lights (`self.Spot Lights`))
  (`|ExecutionSequence`
    (:`then_0`
      ;[1 1 1] Add user-defined Lights
      (for _array_element (`self.🚦 Additional Traffic Lights`)
        (`self.Add one Traffic Light mesh` (`KismetMathLibrary.MakeTransform` (.location _array_element) (.rotation _array_element) (/ (.scale _array_element) _returnvalue)))))
    (:`then_1`
      (for _array_element_2 (`self.🚦 Additional Pedestrian Lights`)
        (`self.Add one Traffic Light mesh` (`KismetMathLibrary.MakeTransform` (.location _array_element_2) (.rotation _array_element_2) (/ (.scale _array_element_2) _returnvalue)) true)))
    (:`then_2`
      ;[1 1 1] Bind each Traffic Light to one of four directions (based on Traffic Light orientation)
      (for (_array_element_3 _array_index) (`self.Traffilc Light Array`)
        (`|ExecutionSequence`
          (:`then_0`
            (bind (_returnvalue_roll _returnvalue_pitch _returnvalue_yaw) (`KismetMathLibrary.BreakRotator` (`KismetMathLibrary.InverseTransformRotation` (`self.GetTransform` self) (`SceneComponent.K2_GetComponentRotation` (break `/Game/Road_Creator_Pro/Blueprints/Helpers/Traffic_Lights` _array_element_3)))))
            (if (`KismetMathLibrary.InRange_FloatFloat` _returnvalue_yaw -135.0 -45.0)
              (set `local.Binding` 0)
              (elif (`KismetMathLibrary.InRange_FloatFloat` _returnvalue_yaw -45.0 45.0)
                (set `local.Binding` 2)
                (elif (`KismetMathLibrary.InRange_FloatFloat` _returnvalue_yaw 45.0 135.0)
                  (set `local.Binding` 1)
                  (else
                    (set `local.Binding` 3))))))
          (:`then_1`
            (bind (_output_mesh _output_binding _output_pedestrian) (break `/Game/Road_Creator_Pro/Blueprints/Helpers/Traffic_Lights` (`|GetArrayItem` _traffilc_light_array _array_index)))
            (`KismetArrayLibrary.Array_Set` _traffilc_light_array _array_index (make `/Game/Road_Creator_Pro/Blueprints/Helpers/Traffic_Lights` _output_mesh (`local.Binding`) _output_pedestrian))))))
    (:`then_3`
      ;[1 1 1] Remove Traffic Lights if this Entry is disabled in "Intersection Entry" array
      (bind _output_get (set `local.Array Length` (- (`KismetArrayLibrary.Array_Length` _traffilc_light_array_2) 1)))
      (for _index (range (+ _output_get 1))
        (bind _returnvalue_2 (- _output_get _index))
        (bind (_output_mesh_2 _output_binding_2 _output_pedestrian_2) (break `/Game/Road_Creator_Pro/Blueprints/Helpers/Traffic_Lights` (`|GetArrayItem` _traffilc_light_array_2 _returnvalue_2)))
        (if _output_pedestrian_2
          _
          (elif (not (`|GetArrayItem` (`self.Intersection Entry`) _output_binding_2))
            (`ActorComponent.K2_DestroyComponent` _output_mesh_2)
            (`KismetArrayLibrary.Array_Remove` (`self.Traffilc Light Array`) _returnvalue_2)
            (if (`self.🚦 Add Spot Lights to Traffic Lights`)
              (`ActorComponent.K2_DestroyComponent` (`|GetArrayItem` _spot_lights _returnvalue_2))
              (`KismetArrayLibrary.Array_Remove` _spot_lights _returnvalue_2))))))))

(fn `Setup Poles and Traffic Lights on them`
  (locals (`Pole Index` :type Integer) (`Current Pole Mesh` :type "StaticMeshComponent Object Reference"))
  (bind _current_pole_mesh (`local.Current Pole Mesh`))
  (bind ___left_hand_drive_for_poles (`self.🚦 Left Hand Drive for Poles`))
  (bind _current_pole_mesh_2 (`local.Current Pole Mesh`))
  (bind _pole_index (`local.Pole Index`))
  (bind _returnvalue (select `bool` ___left_hand_drive_for_poles :`false` (`self.🚦 Poles on Exit`) :`true` (`self.🚦 Poles on Entry`)))
  (`|ExecutionSequence`
    (:`then_0`
      ;[1 1 1] Setup Poles
      (bind _output_get (set `self.Poles Array` (`|MakeArray` (`self.Pole A Entry`) (`self.Pole B Entry`) (`self.Pole C Entry`) (`self.Pole D Entry`) (`self.Pole A Exit`) (`self.Pole B Exit`) (`self.Pole C Exit`) (`self.Pole D Exit`))))
      (for (_array_element _array_index) _output_get
        (set `local.Pole Index` _array_index)
        (if (`self.🚦 Poles`)
          (if (select `bool` (and (`|EnumEquality` (`self.Intersection Type`) "NewEnumerator6") (select `int` (`local.Pole Index`) :`0` false :`1` false :`2` true :`3` true :`4` false :`5` false :`6` true :`7` true)) :`false` (select `bool` (select `bool` ___left_hand_drive_for_poles :`false` (`self.🚦 Poles on Entry`) :`true` (`self.🚦 Poles on Exit`)) :`false` (select `bool` _returnvalue :`false` (select `int` _pole_index :`0` false :`1` false :`2` false :`3` false :`4` false :`5` false :`6` false :`7` false) :`true` (select `int` _pole_index :`0` false :`1` false :`2` false :`3` false :`4` true :`5` true :`6` true :`7` true)) :`true` (select `bool` _returnvalue :`false` (select `int` _pole_index :`0` true :`1` true :`2` true :`3` true :`4` false :`5` false :`6` false :`7` false) :`true` (select `int` _pole_index :`0` true :`1` true :`2` true :`3` true :`4` true :`5` true :`6` true :`7` true))))
            (`KismetArrayLibrary.Array_Add` (`self.Poles`) _array_element)
            (else
              (`ActorComponent.K2_DestroyComponent` _array_element :!label _label)))
          (else
            (goto _label)))))
    (:`then_1`
      ;[1 1 1] For each Pole, add Traffic Lights to needed sockets
      (for _array_element_2 (`self.Poles`)
        (set `local.Current Pole Mesh` _array_element_2)
        (if (`self.🚦 Overhead Poles`)
          (`StaticMeshComponent.SetStaticMesh` _array_element_2 "/Game/Road_Creator_Pro/Meshes/Intersection/SM_Pole_Overhead.SM_Pole_Overhead")
          (if (`self.🚦 Left Hand Drive for Poles`)
            (`SceneComponent.SetRelativeScale3D` _array_element_2 (-1.0 1.0 1.0))))
        (for _array_element_3 (`SceneComponent.GetAllSocketNames` _current_pole_mesh)
          (bind _returnvalue_2 (`KismetStringLibrary.Conv_NameToString` _array_element_3))
          (bind _returnvalue_3 (`KismetStringLibrary.Contains` _returnvalue_2 "Ped"))
          (if (or (and (`self.🚦 Traffic Lights at back of Entry Poles`) (xor (`KismetStringLibrary.Contains` (`KismetSystemLibrary.GetObjectName` _current_pole_mesh) "Entry") (`self.🚦 Left Hand Drive for Poles`)) (`KismetStringLibrary.Contains` _returnvalue_2 "TL")) (`KismetStringLibrary.Contains` _returnvalue_2 "Front") (and _returnvalue_3 (`self.🚦 Pedestrian Lights`)))
            (if _returnvalue_3
              (if (> (`KismetMathLibrary.Dot_VectorVector` (`KismetMathLibrary.GetRightVector` (`SceneComponent.GetSocketRotation` _current_pole_mesh_2 _array_element_3)) (`KismetMathLibrary.GetForwardVector` (`KismetMathLibrary.FindLookAtRotation` (`SceneComponent.GetSocketLocation` _current_pole_mesh_2 _array_element_3) (`self.K2_GetActorLocation`)))) 0.0)
                (bind _mesh (`self.Add one Traffic Light mesh` (struct) _returnvalue_3 :!label _label_2))
                (`SceneComponent.K2_AttachToComponent` _mesh (`local.Current Pole Mesh`) _array_element_3 "KeepRelative" "KeepRelative" "KeepRelative" true)
                (if (and (`KismetStringLibrary.Contains` _returnvalue_2 "Up") (`self.🚥 Horizontal upper Traffic Lights`))
                  (`StaticMeshComponent.SetStaticMesh` _mesh "/Game/Road_Creator_Pro/Meshes/Intersection/SM_Traffilc_Light_Horizontal.SM_Traffilc_Light_Horizontal")))
              (else
                (goto _label_2)))))))))

(fn `Switch Intersection State`
  (bind ___yellow___yellow_red_time (`self.🕚 Yellow / Yellow+Red Time`))
  (bind _current_way (`self.Current Way`))
  (bind _stop_zone_light (`self.Stop Zone Light`))
  (bind _returnvalue (select `/Game/Road_Creator_Pro/Blueprints/Helpers/Current_Way` (`self.Current Way`) :`NewEnumerator1` 2 :`NewEnumerator3` 1 :`NewEnumerator4` 2 :`NewEnumerator5` 3))
  (bind _output (`|GetArrayItem` (`self.Stop Zone Light`) _returnvalue))
  (bind _returnvalue_2 (+ _output 1))
  ;[1 1 1] Timing
  (bind _result (`/Engine/EditorBlueprintResources/StandardMacros.IncrementInt` (`self.Time Elapsed`))
    (:`  `
      (if (>= _result (select `int` _output :`0` (`self.🕑 Green Time`) :`1` ___yellow___yellow_red_time :`2` (`self.🕒 All Red Time`) :`3` ___yellow___yellow_red_time))
        (set `self.Time Elapsed` 0)
        (`KismetArrayLibrary.Array_Set` _stop_zone_light _returnvalue (select `bool` (> _returnvalue_2 (`self.Maximum Light num`)) :`false` _returnvalue_2))
        (if (or (`|EnumEquality` _current_way "NewEnumerator0") (`|EnumEquality` _current_way "NewEnumerator1"))
          (`KismetArrayLibrary.Array_Set` _stop_zone_light (+ _returnvalue 1) (`|GetArrayItem` _stop_zone_light _returnvalue)))
        (if (== (`|GetArrayItem` (`self.Stop Zone Light`) _returnvalue) 2)
          (set `self.Current Way` (select `/Game/Road_Creator_Pro/Blueprints/Helpers/Current_Way` (`self.Current Way`) :`NewEnumerator0` (select `bool` (`self.2-way Intersection`) :`false` "NewEnumerator1" :`true` "NewEnumerator0" :!type "/Game/Road_Creator_Pro/Blueprints/Helpers/Current_Way Enum") :`NewEnumerator1` "NewEnumerator0" :`NewEnumerator2` "NewEnumerator3" :`NewEnumerator3` "NewEnumerator4" :`NewEnumerator4` "NewEnumerator5" :`NewEnumerator5` "NewEnumerator2") :!label _label)
          (`|ExecutionSequence`
            (:`then_0`
              (if (`|EnumEquality` (`self.Intersection Type`) "NewEnumerator1")
                (if (`|GetArrayItem` (`self.Intersection Entry`) (select `/Game/Road_Creator_Pro/Blueprints/Helpers/Current_Way` (`self.Current Way`) :`NewEnumerator3` 1 :`NewEnumerator4` 2 :`NewEnumerator5` 3))
                  _
                  (else
                    (goto _label))))
              (if (== (`self.🕒 All Red Time`) 0)
                (`|ExecutionSequence`
                  (:`then_0`
                    (`self.Switch Intersection State`))
                  (:`then_1`
                    (`self.Update And Traffic Lights` :!label _label_2)))
                (else
                  (goto _label_2)))))
          (else
            (goto _label_2)))))))

(fn `Update And Traffic Lights`
  (locals (Index :type Integer))
  (bind _stop_zone_light (`self.Stop Zone Light`))
  (bind _output (`|GetArrayItem` (`self.Stop Zone Light`) (`local.Index`)))
  (bind _returnvalue (> (`local.Index`) 1))
  (bind _output_2 (`|GetArrayItem` _stop_zone_light (`KismetMathLibrary.SelectInt` 2 0 _returnvalue)))
  (bind _output_3 (`|GetArrayItem` _stop_zone_light (`KismetMathLibrary.SelectInt` 3 1 _returnvalue)))
  (bind _returnvalue_2 (and (!= _output_2 1) (!= _output_2 3) (!= _output_3 1) (!= _output_3 3) (== (`|GetArrayItem` _stop_zone_light (`KismetMathLibrary.SelectInt` 0 2 _returnvalue)) 2) (== (`|GetArrayItem` _stop_zone_light (`KismetMathLibrary.SelectInt` 1 3 _returnvalue)) 2)))
  ;[1 1 1] Update Traffic Lights
  (for (_array_element _array_index) (`self.Traffilc Light Array`)
    (set `local.Index` (`.Binding_6_1591385B49A2B32454319D8D9483E406` (break `/Game/Road_Creator_Pro/Blueprints/Helpers/Traffic_Lights` _array_element)))
    (if (`.Pedestrian_9_1B91CA164BC1AEAC934A1199771640A4` (break `/Game/Road_Creator_Pro/Blueprints/Helpers/Traffic_Lights` _array_element))
      (`MeshComponent.SetScalarParameterValueOnMaterials` (break `/Game/Road_Creator_Pro/Blueprints/Helpers/Traffic_Lights` _array_element) "Red" (`KismetMathLibrary.Conv_BoolToDouble` (not _returnvalue_2)))
      (`MeshComponent.SetScalarParameterValueOnMaterials` (break `/Game/Road_Creator_Pro/Blueprints/Helpers/Traffic_Lights` _array_element) "Green" (`KismetMathLibrary.Conv_BoolToDouble` _returnvalue_2))
      ;[1 1 1] Update Spot Lights
      (if (`self.🚦 Add Spot Lights to Traffic Lights`)
        (bind _output_4 (`|GetArrayItem` (`self.Spot Lights`) _array_index))
        (`LightComponent.SetLightColor` _output_4 (`KismetMathLibrary.SelectColor` (struct :`G` 1.0 :`A` 1.0) (struct :`R` 1.0 :`A` 1.0) _returnvalue_2) true))
      (else
        (`MeshComponent.SetScalarParameterValueOnMaterials` (break `/Game/Road_Creator_Pro/Blueprints/Helpers/Traffic_Lights` _array_element) "Red" (select `int` _output :`0` 0.0 :`1` 0.0 :`2` 1.0 :`3` 1.0 :!type "Float (single-precision)"))
        (`MeshComponent.SetScalarParameterValueOnMaterials` (break `/Game/Road_Creator_Pro/Blueprints/Helpers/Traffic_Lights` _array_element) "Yellow" (select `int` _output :`0` 0.0 :`1` 1.0 :`2` 0.0 :`3` 1.0 :!type "Float (single-precision)"))
        (`MeshComponent.SetScalarParameterValueOnMaterials` (break `/Game/Road_Creator_Pro/Blueprints/Helpers/Traffic_Lights` _array_element) "Green" (select `int` _output :`0` 1.0 :`1` 0.0 :`2` 0.0 :`3` 0.0 :!type "Float (single-precision)"))
        (if (`self.🚦 Add Spot Lights to Traffic Lights`)
          (`LightComponent.SetLightColor` _output_4 (select `int` _output :`0` (struct :`G` 1.0 :`A` 1.0) :`1` (struct :`R` 1.0 :`G` 1.0 :`A` 1.0) :`2` (struct :`R` 1.0 :`A` 1.0) :`3` (struct :`R` 1.5 :`G` 0.677088 :`A` 1.0) :!type "LinearColor Structure") true))))))

(fn `UserConstructionScript`
  (bind _starting_state (`self.Starting State`))
  (bind _stop_zone_light (`self.Stop Zone Light`))
  (bind _starting_state_2 (`self.Starting State`))
  (bind _starting_state_3 (`self.Starting State`))
  (bind _two_ways_at_a_time (`self.Two Ways at a time`))
  (bind _texts_array (`self.Texts Array`))
  (bind _intersection_type (`self.Intersection Type`))
  (bind _returnvalue (`|EnumEquality` _starting_state_2 "NewEnumerator1"))
  (bind _returnvalue_2 (`|EnumEquality` _starting_state_2 "NewEnumerator3"))
  (bind _returnvalue_3 (`|EnumEquality` _starting_state_2 "NewEnumerator2"))
  (bind _returnvalue_4 (`|EnumEquality` _starting_state_2 "NewEnumerator4"))
  (bind _returnvalue_5 (or _returnvalue_2 _returnvalue_4))
  (bind _returnvalue_6 (or _returnvalue _returnvalue_3))
  (`|ExecutionSequence`
    (:`then_0`
      ;[1 1 1] Intersection Type
      (set `self.Two Ways at a time` (select `/Game/Road_Creator_Pro/Blueprints/Helpers/Intersection_Types_Simple` _intersection_type :`NewEnumerator0` true :`NewEnumerator6` true))
      (set `self.2-way Intersection` (`|EnumEquality` _intersection_type "NewEnumerator6")))
    (:`then_1`
      ;[1 1 1] Texts
      (set `self.Texts Array` (`|MakeArray` (`self.Text A`) (`self.Text B`) (`self.Text C`) (`self.Text D`)))
      (`|ExecutionSequence`
        (:`then_1`
          (if (`self.2-way Intersection`)
            (`ActorComponent.K2_DestroyComponent` (`self.Text C`))
            (`ActorComponent.K2_DestroyComponent` (`self.Text D`))))
        (:`then_2`
          (for (_array_element _array_index) _texts_array
            (`/Engine/EditorBlueprintResources/StandardMacros.IsValid` _array_element
              (:`Is Valid`
                (if (not (`|GetArrayItem` (`self.Intersection Entry`) _array_index))
                  (`ActorComponent.K2_DestroyComponent` (`|GetArrayItem` _texts_array _array_index)))))))))
    (:`then_3`
      ;[1 1 1] Whether to use Red+Yellow light
      (set `self.Maximum Light num` (`KismetMathLibrary.SelectInt` 3 2 (`self.European Lights Sequence`)))
      ;[1 1 1] Disable Green D default state for 3-way intersection
      (if (and (or (`|EnumEquality` _starting_state "NewEnumerator4") (`|EnumEquality` _starting_state "NewEnumerator3")) (`self.2-way Intersection`))
        (set `self.Starting State` "NewEnumerator0")))
    (:`then_4`
      ;[1 1 1] Starting State of Traffic Lights
      (`KismetArrayLibrary.Array_Set` _stop_zone_light 0 (`KismetMathLibrary.SelectInt` 0 2 (select `bool` _two_ways_at_a_time :`false` _returnvalue :`true` _returnvalue_6)))
      (`KismetArrayLibrary.Array_Set` _stop_zone_light 1 (`KismetMathLibrary.SelectInt` 0 2 (select `bool` _two_ways_at_a_time :`false` _returnvalue_3 :`true` _returnvalue_6)))
      (`KismetArrayLibrary.Array_Set` _stop_zone_light 2 (`KismetMathLibrary.SelectInt` 0 2 (select `bool` (`self.Two Ways at a time`) :`false` _returnvalue_2 :`true` _returnvalue_5)))
      (`KismetArrayLibrary.Array_Set` _stop_zone_light 3 (`KismetMathLibrary.SelectInt` 0 2 (select `bool` (`self.Two Ways at a time`) :`false` _returnvalue_4 :`true` _returnvalue_5)))
      (set `self.Current Way` (select `bool` (`self.Two Ways at a time`) :`false` (select `/Game/Road_Creator_Pro/Blueprints/Helpers/Starting_State` _starting_state_3 :`NewEnumerator0` "NewEnumerator2" :`NewEnumerator1` "NewEnumerator2" :`NewEnumerator2` "NewEnumerator3" :`NewEnumerator3` "NewEnumerator4" :`NewEnumerator4` "NewEnumerator5" :!type "/Game/Road_Creator_Pro/Blueprints/Helpers/Current_Way Enum") :`true` (select `/Game/Road_Creator_Pro/Blueprints/Helpers/Starting_State` _starting_state_3 :`NewEnumerator0` "NewEnumerator0" :`NewEnumerator1` "NewEnumerator0" :`NewEnumerator2` "NewEnumerator0" :`NewEnumerator3` "NewEnumerator1" :`NewEnumerator4` "NewEnumerator1" :!type "/Game/Road_Creator_Pro/Blueprints/Helpers/Current_Way Enum"))))
    (:`then_5`
      (`|ExecutionSequence`
        (:`then_0`
          (`self.Setup Poles and Traffic Lights on them`))
        (:`then_1`
          (`self.Add Traffic LIghts And Bind Them`)
          (`self.Update And Traffic Lights`))))
    (:`then_6`
      (set `self.❓Hover for Help ` false))))